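; T90 tank Blueprint that handles player input for driving, camera aiming and firing.
; On BeginPlay it hands the barrel and turret to the T90Aiming component and both tracks to T90Movement.
; Throttle axes drive each track directly, while forward and turn axes go through T90Movement as intents.
; Aim axes rotate the azimuth gimbal and spring arm, scaled by delta time, and Fire calls T90Aiming.
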(event `self.ReceiveBeginPlay`
  (`T90AimingComponent.Initialize` (`self.T90Aiming`) (`self.T90Barrel`) (`self.T90Turret`))
  (`T90MovementComponent.Initialize` (`self.T90Movement`) (`self.LeftTrack`) (`self.RightTrack`)))

(event `InputAxis|Left Track Throttle`
  (params (AxisValue :type "Float (single-precision)"))
  ;[1 1 1] 输入控制移动
  (`T90Track.SetThrottle` (`self.LeftTrack`) AxisValue))

(event `InputAxis|AimAzimuth`
  (params (AxisValue :type "Float (single-precision)"))
  ;[1 1 1] 输入控制瞄准与射击
  (`SceneComponent.K2_AddLocalRotation` (`self.Azimuth Gimbal`) (`KismetMathLibrary.MakeRotator` 0.0 0.0 (* AxisValue (`GameplayStatics.GetWorldDeltaSeconds`) 50.0)) false false))

(event `InputAxis|Right Track Throttle`
  (params (AxisValue :type "Float (single-precision)"))
  ;[1 1 1] 输入控制移动
  (`T90Track.SetThrottle` (`self.RightTrack`) AxisValue))

(event `InputAxis|AimElevation`
  (params (AxisValue :type "Float (single-precision)"))
  ;[1 1 1] 输入控制瞄准与射击
  (`SceneComponent.K2_AddLocalRotation` (`self.SpringArm`) (`KismetMathLibrary.MakeRotator` 0.0 (* AxisValue (`GameplayStatics.GetWorldDeltaSeconds`) 20.0)) false false))

(event `InputAxis|Move Forward`
  (params (AxisValue :type "Float (single-precision)"))
  ;[1 1 1] 输入控制移动
  (`T90MovementComponent.IntendMoveForward` (`self.T90Movement`) AxisValue))

(event `InputAction|Fire`
  (params (Key :type "Key Structure" :default "AnyKey"))
  ;[1 1 1] 输入控制瞄准与射击
  (:`Pressed`
    (`T90AimingComponent.Fire` (`self.T90Aiming`))))

(event `InputAxis|Turn Right`
  (params (AxisValue :type "Float (single-precision)"))
  ;[1 1 1] 输入控制移动
  (`T90MovementComponent.IntendTurnRight` (`self.T90Movement`) AxisValue))

(fn `UserConstructionScript`)